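; BP_Hatch_01 is a sci-fi corridor hatch that opens when anything overlaps its Box trigger and closes when the overlap ends.
; The Door_Slide timeline drives the relative roll of SMHatch01B, playing on begin overlap and reversing on end overlap.
; At BeginPlay, MyLever attaches to that moving mesh, keeping its world transform.
; The construction script applies the Material variable to both hatch meshes.
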(event OnComponentBeginOverlap(Box)
  (params (OverlappedComponent :type Primitive%20Component%20Object%20Reference) (OtherActor :type Actor%20Object%20Reference) (OtherComp :type Primitive%20Component%20Object%20Reference) (OtherBodyIndex :type Integer) (bFromSweep :type Boolean) (SweepResult :type Hit%20Result%20Structure%20%28by%20ref%29))
  (bind _newtrack_0 (Timeline|Door_Slide Play)
    (:Update
      (Transformation|SetRelativeRotation (Variables|Default|GetSM_Hatch_01_B) (Math|Rotator|MakeRotator _newtrack_0 0.0 0.0) false false))))

(event OnComponentEndOverlap(Box)
  (params (OverlappedComponent :type Primitive%20Component%20Object%20Reference) (OtherActor :type Actor%20Object%20Reference) (OtherComp :type Primitive%20Component%20Object%20Reference) (OtherBodyIndex :type Integer))
  (bind _newtrack_0 (Timeline|Door_Slide Reverse)
    (:Update
      (Transformation|SetRelativeRotation (Variables|Default|GetSM_Hatch_01_B) (Math|Rotator|MakeRotator _newtrack_0 0.0 0.0) false false))))

(event EventBeginPlay
  (Transformation|AttachComponentToComponent (Variables|Default|GetMyLever) (Variables|Default|GetSM_Hatch_01_B) "None" "KeepWorld" "KeepWorld" "KeepWorld" true))

(fn ConstructionScript
  (Rendering|Material|SetMaterial (Variables|Default|GetSM_Hatch_01_A) 0 (Variables|Default|GetMaterial)))