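; Orange lever for a Stage 3 door, an interactable that toggles the lock on its target door and triggers a room move.
; A FlipFlop on OnInteract alternates between locking the door while starting the target room's move, and unlocking the door without calling the room.
; The TL_Lever timeline plays on the first state and reverses on the second, lerping the lever pivot's roll to animate the handle.
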(event EventBeginPlay)

(event Collision|EventActorBeginOverlap
  (params (OtherActor :type Actor%20Object%20Reference)))

(event EventTick
  (params (DeltaSeconds :type Float%20%28single-precision%29)))

(event EventOnInteract
  (bind _targetdoor (Variables|Default|GetTargetDoor))
  (Utilities|FlowControl|FlipFlop
    (:A
      (Variables|/Game/PersonalProject/Blueprint/Stage3/BP_Door1_Locked_Orange.BP_Door1_Locked_Orange_C|SetIsLocked _targetdoor true)
      (Default|StartMove (Variables|Default|GetTargetRoom))
      (bind _alpha (Timeline|TL_Lever Play)
        (:Update
          (Transformation|SetRelativeRotation (Variables|Default|GetLeverPivot) (Math|Rotator|MakeRotator (Math|Float|Lerp -1e+02 (Variables|Default|GetLeverOpenRotation) _alpha) 0.0 0.0) false false))))
    (:B
      (Variables|/Game/PersonalProject/Blueprint/Stage3/BP_Door1_Locked_Orange.BP_Door1_Locked_Orange_C|SetIsLocked _targetdoor false)
      (Timeline|TL_Lever Reverse))))

(fn ConstructionScript)