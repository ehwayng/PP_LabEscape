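; BP_LeverRoom is a Stage 3 room actor that moves continuously until told to stop and slide to a set position.
; On BeginPlay, TL_MovingRoom starts, offsetting height from the initial location by RoomTilt and setting yaw from RoomRotate.
; StopAndMoveToStart stops that timeline, then TL_MoveToStart lerps from the current location to a hardcoded point, leaving rotation as is.
; The saved InitialRotation is never used.
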(event Custom|StopAndMoveToStart
  (Utilities|FlowControl|Sequence
    (:then_0
      (bind (_direction _roomtilt _roomrotate) (Timeline|TL_MovingRoom Stop)
        (:Update
          (Transformation|SetActorLocationAndRotation (+ (Math|Vector|MakeVector 0.0 0.0 _roomtilt) (Variables|Default|GetInitialLocation)) (Math|Rotator|MakeRotator 0.0 0.0 _roomrotate)))))
    (:then_1
      (Variables|Default|SetCurrentLocation (Transformation|GetActorLocation))
      (bind _movetostart (Timeline|TL_MoveToStart PlayFromStart)
        (:Update
          (Transformation|SetActorLocation (Math|Vector|Lerp(Vector) (Variables|Default|GetCurrentLocation) "4230.000000,-210.000000,90.000000" _movetostart) false false))))))

(event EventBeginPlay
  (Variables|Default|SetInitialLocation (Transformation|GetActorLocation))
  (Variables|Default|SetInitialRotation (Transformation|GetActorRotation))
  (bind (_direction _roomtilt _roomrotate) (Timeline|TL_MovingRoom Play)
    (:Update
      (Transformation|SetActorLocationAndRotation (+ (Math|Vector|MakeVector 0.0 0.0 _roomtilt) (Variables|Default|GetInitialLocation)) (Math|Rotator|MakeRotator 0.0 0.0 _roomrotate)))))

(fn ConstructionScript)