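; Stage 3 hell tunnel actor that rolls its TunnelPivot with a timeline when TunnelRotate is called.
; The GravityReverse flag selects whether TL_Gravity plays from start or reverses from end.
; GravityZone overlap events are empty.
; Disconnected logic would flip BP_Player gravity upward on entry and use a TunnelCount counter to restore it after leaving the last zone.
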(event OnComponentBeginOverlap(GravityZone)
  (params (OverlappedComponent :type Primitive%20Component%20Object%20Reference) (OtherActor :type Actor%20Object%20Reference) (OtherComp :type Primitive%20Component%20Object%20Reference) (OtherBodyIndex :type Integer) (bFromSweep :type Boolean) (SweepResult :type Hit%20Result%20Structure%20%28by%20ref%29))
  ;[0.15 0.15 0.15 0.5] 플레이어 진입시 중력 반전 / 탈출시 원상복구
)

(event OnComponentEndOverlap(GravityZone)
  (params (OverlappedComponent :type Primitive%20Component%20Object%20Reference) (OtherActor :type Actor%20Object%20Reference) (OtherComp :type Primitive%20Component%20Object%20Reference) (OtherBodyIndex :type Integer))
  ;[0.15 0.15 0.15 0.5] 플레이어 진입시 중력 반전 / 탈출시 원상복구
)

(event Custom|TunnelRotate
  (if (Variables|Default|GetGravityReverse)
    (bind _alpha (Timeline|TL_Gravity PlayFromStart)
      (:Update
        (Transformation|SetRelativeRotation (Variables|Default|GetTunnelPivot) (Math|Rotator|MakeRotator _alpha 0.0 0.0) false false)))
    (else
      (Timeline|TL_Gravity ReverseFromEnd))))

(fn ConstructionScript)