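; BP_GlassWall_Floor is a two-panel sliding wall that opens and closes through its OpenWall and CloseWall events.
; OpenWall plays the Door_Slide timeline and CloseWall reverses it.
; The timeline's update lerps the left and right door meshes between stored closed and open relative locations, without sweep.
; The Blueprint has no trigger logic of its own, as BeginPlay, overlap and Tick are unused.
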(event Custom|OpenWall
  (bind _newtrack_0 (Timeline|Door_Slide Play)
    (:Update
      (Transformation|SetRelativeLocation (Variables|Default|GetSM_Door_02_B_Left) (Math|Vector|Lerp(Vector) (Variables|Default|GetDoor_Closed_Left) (Variables|Default|GetDoor_Open_Left) _newtrack_0) false false)
      (Transformation|SetRelativeLocation (Variables|Default|GetSM_Door_02_C_Right) (Math|Vector|Lerp(Vector) (Variables|Default|GetDoor_Closed_Right) (Variables|Default|GetDoor_Open_Right) _newtrack_0) false false))))

(event Custom|CloseWall
  (bind _newtrack_0 (Timeline|Door_Slide Reverse)
    (:Update
      (Transformation|SetRelativeLocation (Variables|Default|GetSM_Door_02_B_Left) (Math|Vector|Lerp(Vector) (Variables|Default|GetDoor_Closed_Left) (Variables|Default|GetDoor_Open_Left) _newtrack_0) false false)
      (Transformation|SetRelativeLocation (Variables|Default|GetSM_Door_02_C_Right) (Math|Vector|Lerp(Vector) (Variables|Default|GetDoor_Closed_Right) (Variables|Default|GetDoor_Open_Right) _newtrack_0) false false))))

(event EventBeginPlay)

(event Collision|EventActorBeginOverlap
  (params (OtherActor :type Actor%20Object%20Reference)))

(event EventTick
  (params (DeltaSeconds :type Float%20%28single-precision%29)))

(fn ConstructionScript)