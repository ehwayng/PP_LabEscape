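; BP_Lever_Tunnel is a Stage 2 interactable lever that switches gravity reversal on a linked tunnel.
; Each interaction alternates through a FlipFlop, setting the target tunnel's GravityReverse flag on or off and calling its TunnelRotate.
; A timeline plays forward or in reverse to swing the lever pivot's roll between its rest angle and LeverOpenRotation.
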(event EventBeginPlay)

(event Collision|EventActorBeginOverlap
  (params (OtherActor :type Actor%20Object%20Reference)))

(event EventTick
  (params (DeltaSeconds :type Float%20%28single-precision%29)))

(event EventOnInteract
  (bind _targettunnel (Variables|Default|GetTargetTunnel))
  (Utilities|FlowControl|FlipFlop
    (:A
      (Variables|/Game/PersonalProject/Blueprint/Stage2/BP_Tunnel.BP_Tunnel_C|SetGravityReverse _targettunnel true)
      (Default|TunnelRotate _targettunnel)
      (bind _alpha (Timeline|TL_Lever Play)
        (:Update
          (Transformation|SetRelativeRotation (Variables|Default|GetLeverPivot) (Math|Rotator|MakeRotator (Math|Float|Lerp -1e+02 (Variables|Default|GetLeverOpenRotation) _alpha) 0.0 0.0) false false))))
    (:B
      (Variables|/Game/PersonalProject/Blueprint/Stage2/BP_Tunnel.BP_Tunnel_C|SetGravityReverse _targettunnel false)
      (Default|TunnelRotate _targettunnel)
      (Timeline|TL_Lever Reverse))))

(fn ConstructionScript)