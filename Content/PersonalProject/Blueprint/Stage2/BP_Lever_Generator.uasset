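; Interactable lever for Stage 2 that switches a linked generator on and off.
; Each interaction flip-flops the activated state, broadcasts a lever state change, then signals the first valid target among generators A, B and C.
; With a valid target, a timeline plays or reverses to roll the lever pivot, re-broadcasting the state change on every update.
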(event EventBeginPlay)

(event Collision|EventActorBeginOverlap
  (params (OtherActor :type Actor%20Object%20Reference)))

(event EventTick
  (params (DeltaSeconds :type Float%20%28single-precision%29)))

(event EventOnInteract
  (bind _targetgena (Variables|Default|GetTargetGenA))
  (bind _targetgenb (Variables|Default|GetTargetGenB))
  (bind _targetgenc (Variables|Default|GetTargetGenC))
  (bind _targetgena_2 (Variables|Default|GetTargetGenA))
  (bind _targetgenb_2 (Variables|Default|GetTargetGenB))
  (bind _targetgenc_2 (Variables|Default|GetTargetGenC))
  (Utilities|FlowControl|FlipFlop
    (:A
      (Variables|Default|SetIsActivated true)
      (Default|CallLeverStateChanged)
      (Utilities|IsValid _targetgena_2
        (:Is%20Valid
          (Default|GenerateAon _targetgena_2)
          (bind _alpha (Timeline|TL_Lever Play)
            (:Update
              (Transformation|SetRelativeRotation (Variables|Default|GetLeverPivot) (Math|Rotator|MakeRotator (Math|Float|Lerp -1e+02 (Variables|Default|GetLeverOpenRotation) _alpha) 0.0 0.0) false false)
              (Default|CallLeverStateChanged))))
        (:Is%20Not%20Valid
          (Utilities|IsValid _targetgenb_2
            (:Is%20Valid
              (Default|GeneratorBon _targetgenb_2)
              (Timeline|TL_Lever Play))
            (:Is%20Not%20Valid
              (Utilities|IsValid _targetgenc_2
                (:Is%20Valid
                  (Default|GeneratorCon _targetgenc_2)
                  (Timeline|TL_Lever Play))))))))
    (:B
      (Variables|Default|SetIsActivated false)
      (Default|CallLeverStateChanged)
      (Utilities|IsValid _targetgena
        (:Is%20Valid
          (Default|GeneratorAOff _targetgena)
          (Timeline|TL_Lever Reverse))
        (:Is%20Not%20Valid
          (Utilities|IsValid _targetgenb
            (:Is%20Valid
              (Default|GeneratorBOff _targetgenb)
              (Timeline|TL_Lever Reverse))
            (:Is%20Not%20Valid
              (Utilities|IsValid _targetgenc
                (:Is%20Valid
                  (Default|GeneratorCOff _targetgenc)
                  (Timeline|TL_Lever Reverse))))))))))

(fn ConstructionScript)