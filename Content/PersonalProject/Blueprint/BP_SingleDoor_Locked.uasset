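; BP_SingleDoor_Locked is a lockable single door that swings away from or toward its front when interacted with.
; OnInteract uses a dot product of the player's direction and the door's forward vector to pick one of two timelines.
; Each timeline lerps DoorPivot yaw from zero to PullDoorRotation or PushDoorRotation, with no closing logic.
; The IsLocked check reads inverted: true opens the door, false prints a locked message.
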(event EventBeginPlay)

(event Collision|EventActorBeginOverlap
  (params (OtherActor :type Actor%20Object%20Reference)))

(event EventTick
  (params (DeltaSeconds :type Float%20%28single-precision%29)))

(event EventOnInteract
  ;[0.15 0.15 0.15 0.5] 문과 플레이어의 상대적 위치
  (if (Variables|Default|GetIsLocked)
    (if (> (Math|Vector|DotProduct (Math|Vector|Normalize (- (Transformation|GetActorLocation (Game|GetPlayerCharacter 0)) (Transformation|GetActorLocation))) (Transformation|GetActorForwardVector)) 0.0)
      ;[0.15 0.15 0.15 0.5] 미시오
      (bind _alpha (Timeline|TL_SingleDoor1 PlayFromStart)
        (:Update
          (Transformation|SetRelativeRotation (Variables|Default|GetDoorPivot) (Math|Rotator|MakeRotator 0.0 0.0 (Math|Float|Lerp 0.0 (Variables|Default|GetPullDoorRotation) _alpha)) false false)))
      (else
        (bind _alpha_2 (Timeline|TL_SingleDoor2 PlayFromStart)
          (:Update
            (Transformation|SetRelativeRotation (Variables|Default|GetDoorPivot) (Math|Rotator|MakeRotator 0.0 0.0 (Math|Float|Lerp 0.0 (Variables|Default|GetPushDoorRotation) _alpha_2)) false false)))))
    (else
      (Development|PrintString "문이 잠겨있습니다! " true true "(R=1.000000,G=0.000000,B=0.059532,A=1.000000)"))))

(fn ConstructionScript)