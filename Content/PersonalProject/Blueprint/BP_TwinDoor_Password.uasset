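; BP_TwinDoor_Password is a keypad-protected double door that swings open relative to the player's side.
; OnInteract shows WBP_KeyPad_forTwin with a reference to the door, switching input to UI-only with a cursor.
; PasswordOpen uses a dot product to pick one of two timelines, rotating both pivots with swapped target angles.
; It opens only when IsLocked is true, despite the name; otherwise it prints a locked message.
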(event Custom|PasswordOpen
  (if (Variables|Default|GetIsLocked)
    (if (> (Math|Vector|DotProduct (Math|Vector|Normalize (- (Transformation|GetActorLocation (Game|GetPlayerCharacter 0)) (Transformation|GetActorLocation))) (Transformation|GetActorForwardVector)) 0.0)
      (bind _alpha (Timeline|TL_TwinDoor1 PlayFromStart)
        (:Update
          (Transformation|SetRelativeRotation (Variables|Default|GetLeftDoorPivot) (Math|Rotator|MakeRotator 0.0 0.0 (Math|Float|Lerp 0.0 (Variables|Default|GetDoorRotation-90) _alpha)) false false)
          (Transformation|SetRelativeRotation (Variables|Default|GetRightDoorPivot) (Math|Rotator|MakeRotator 0.0 0.0 (Math|Float|Lerp 0.0 (Variables|Default|GetDoorRotaion+90) _alpha)) false false)))
      (else
        (bind _alpha_2 (Timeline|TL_TwinDoor2 PlayFromStart)
          (:Update
            (Transformation|SetRelativeRotation (Variables|Default|GetLeftDoorPivot) (Math|Rotator|MakeRotator 0.0 0.0 (Math|Float|Lerp 0.0 (Variables|Default|GetDoorRotaion+90) _alpha_2)) false false)
            (Transformation|SetRelativeRotation (Variables|Default|GetRightDoorPivot) (Math|Rotator|MakeRotator 0.0 0.0 (Math|Float|Lerp 0.0 (Variables|Default|GetDoorRotation-90) _alpha_2)) false false)))))
    (else
      (Development|PrintString "문이 잠겨있습니다! " true true "(R=1.000000,G=0.000000,B=0.059532,A=1.000000)"))))

(event EventBeginPlay)

(event Collision|EventActorBeginOverlap
  (params (OtherActor :type Actor%20Object%20Reference)))

(event EventTick
  (params (DeltaSeconds :type Float%20%28single-precision%29)))

(event EventOnInteract
  (bind _returnvalue (Game|GetPlayerController 0))
  (bind _returnvalue_2 (UserInterface|CreateWidget "/Game/PersonalProject/Blueprint/WBP_KeyPad_forTwin.WBP_KeyPad_forTwin_C" 0 self))
  (UserInterface|Viewport|AddtoViewport _returnvalue_2 0)
  (Variables|/Script/Engine.PlayerController|SetbShowMouseCursor _returnvalue true)
  (Input|SetInputModeUIOnly _returnvalue 0 "DoNotLock" false))

(fn ConstructionScript)