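; BP_TwinDoor is an interactable double door that swings its two leaves on pivots when OnInteract fires.
; A dot product between the door's forward vector and the direction to the player picks one of two timelines by side.
; Each timeline lerps both pivots' yaw from zero, with the two near-identically named rotation variables swapped between branches.
; Every interaction plays from the start, with no closing logic.
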(event EventBeginPlay)

(event Collision|EventActorBeginOverlap
  (params (OtherActor :type Actor%20Object%20Reference)))

(event EventTick
  (params (DeltaSeconds :type Float%20%28single-precision%29)))

(event EventOnInteract
  (if (> (Math|Vector|DotProduct (Math|Vector|Normalize (- (Transformation|GetActorLocation (Game|GetPlayerCharacter 0)) (Transformation|GetActorLocation))) (Transformation|GetActorForwardVector)) 0.0)
    (bind _alpha (Timeline|TL_TwinDoor1 PlayFromStart)
      (:Update
        (Transformation|SetRelativeRotation (Variables|Default|GetLeftDoorPivot) (Math|Rotator|MakeRotator 0.0 0.0 (Math|Float|Lerp 0.0 (Variables|Default|GetDoorRotation-90) _alpha)) false false)
        (Transformation|SetRelativeRotation (Variables|Default|GetRightDoorPivot) (Math|Rotator|MakeRotator 0.0 0.0 (Math|Float|Lerp 0.0 (Variables|Default|GetDoorRotaion+90) _alpha)) false false)))
    (else
      (bind _alpha_2 (Timeline|TL_TwinDoor2 PlayFromStart)
        (:Update
          (Transformation|SetRelativeRotation (Variables|Default|GetLeftDoorPivot) (Math|Rotator|MakeRotator 0.0 0.0 (Math|Float|Lerp 0.0 (Variables|Default|GetDoorRotaion+90) _alpha_2)) false false)
          (Transformation|SetRelativeRotation (Variables|Default|GetRightDoorPivot) (Math|Rotator|MakeRotator 0.0 0.0 (Math|Float|Lerp 0.0 (Variables|Default|GetDoorRotation-90) _alpha_2)) false false))))))

(fn ConstructionScript)